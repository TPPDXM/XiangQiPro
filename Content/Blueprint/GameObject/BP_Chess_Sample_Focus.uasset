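; Clickable chess piece on the main map whose first touch or click sends the start-game message to all MainMapInterface actors and widgets.
; That touch starts timelines that rotate the actor and move the mesh vertically, while another timeline drives the base yaw.
; A DoOnce, reset when the move finishes, lets later touches or a loop macro replay both animations, then swap in a random decal material after a short delay.
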(event `self.ReceiveBeginPlay`
  (set `self.DefaultRotation` (`self.K2_GetActorRotation`))
  (set `self.DefaultLocation` (`SceneComponent.K2_GetComponentLocation` (`self.ChessMesh`))))

(event `self.ChessMesh.OnInputTouchBegin`
  (params (FingerIndex :type "ETouchIndex Enum" :default "Touch1") (TouchedComponent :type "PrimitiveComponent Object Reference"))
  (bind (_defaultrotation_roll _defaultrotation_pitch _defaultrotation_yaw) (`KismetMathLibrary.BreakRotator` (`self.DefaultRotation`)))
  (bind (_defaultlocation_x _defaultlocation_y _defaultlocation_z) (`KismetMathLibrary.BreakVector` (`self.DefaultLocation`)))
  (bind (_defaultrotation_roll_2 _defaultrotation_pitch_2) (`KismetMathLibrary.BreakRotator` (`self.DefaultRotation`)))
  (if (`self.FirstClick`) :!label _label
    (`|ExecutionSequence`
      (:`then_0`
        (bind (_direction `_旋转`) (`Timeline|旋转` :!via `PlayFromStart` :!label _label_2)
          (:`Update`
            (`self.K2_SetActorRotation` (`KismetMathLibrary.MakeRotator` _defaultrotation_roll _defaultrotation_pitch (+ _defaultrotation_yaw `_旋转`))))))
      (:`then_1`
        (bind (_direction_2 `_位置`) (`Timeline|位置` :!via `PlayFromStart` :!label _label_3)
          (:`Update`
            (`SceneComponent.K2_SetWorldLocation` (`self.ChessMesh`) (`KismetMathLibrary.MakeVector` _defaultlocation_x _defaultlocation_y (+ `_位置` _defaultlocation_z)) false false))
          (:`Finished`
            (goto _label_4 :!via `Reset`))))
      (:`then_2`
        (`/Game/Blueprint/LoopMacro.WhileLoopWithBreakAndBreak` 15.0
          (:`Exec`
            (`/Engine/EditorBlueprintResources/StandardMacros.DoOnce` true :!label _label_4
              (:`Completed`
                (`|ExecutionSequence`
                  (:`then_0`
                    (goto _label_2 :!via `PlayFromStart`))
                  (:`then_1`
                    (goto _label_3 :!via `PlayFromStart`))
                  (:`then_2`
                    (`KismetSystemLibrary.Delay` 0.2)
                    (`DecalComponent.SetDecalMaterial` (`self.Decal`) (`KismetArrayLibrary.Array_Random` (`self.DecalList`))))))))))
      (:`then_3`
        (bind (_direction_3 `_z轴旋转`) (`Timeline|Z轴旋转`)
          (:`Update`
            (set `self.DefaultRotation` (`KismetMathLibrary.MakeRotator` _defaultrotation_roll_2 _defaultrotation_pitch_2 `_z轴旋转`)))))
      (:`then_4`
        (bind _outactors (`GameplayStatics.GetAllActorsWithInterface` "/Game/Blueprint/MainMapInterface.MainMapInterface_C"))
        (for _array_element _outactors
          (message `/Game/Blueprint/MainMapInterface.TouchToStartGame` _array_element))
        (bind _foundwidgets (`WidgetBlueprintLibrary.GetAllWidgetsWithInterface` "/Game/Blueprint/MainMapInterface.MainMapInterface_C" true))
        (for _array_element_2 _foundwidgets
          (message `/Game/Blueprint/MainMapInterface.TouchToStartGame` _array_element_2))
        (set `self.FirstClick` false)))
    (else
      (goto _label_4))))

(event `self.ChessMesh.OnClicked`
  (params (TouchedComponent :type "PrimitiveComponent Object Reference") (ButtonPressed :type "Key Structure"))
  (goto _label))

(fn `UserConstructionScript`
  (`parent.UserConstructionScript`))